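; Basic snowman enemy for an FPS that throws projectiles at the player when it sees them.
; When PawnSensing spots a BP_FPSCharacter, it instantly turns to face that character.
; It then spawns a BP_Projectile at SnowBallSpawnPoint, with a CanAttack flag and a one-second delay limiting the fire rate.
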(event OnSeePawn(PawnSensing)
  (params (Pawn :type Pawn%20Object%20Reference))
  (bind _asbp_fpscharacter (Utilities|Casting|CastToBP_FPSCharacter Pawn))
  (Transformation|SetActorRotation (Math|Rotator|FindRelativeLookatRotation (Math|Conversions|ToTransform(Vector) (Transformation|GetActorLocation)) (Transformation|GetActorLocation _asbp_fpscharacter)))
  (if (Variables|Default|GetCanAttack)
    (Game|SpawnActorfromClass "/Game/FPS/Blueprint/Guns/BP_Projectile.BP_Projectile_C" (Transformation|GetWorldTransform (Variables|Default|GetSnowBallSpawnPoint)) "Undefined" "MultiplyWithRoot" 0 0)
    (Variables|Default|SetCanAttack false)
    (Utilities|FlowControl|Delay 1.0)
    (Variables|Default|SetCanAttack true)))

(fn ConstructionScript)