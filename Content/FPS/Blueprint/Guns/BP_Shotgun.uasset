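; Player shotgun Blueprint that fires snowball projectiles as a single shot or a six-point spread, extending parent gun shoot and reload logic.
; Single shots cost one ammo, spreads cost twelve, and the player's AmmoAbility usually skips that cost.
; CritAbility ties crit chance to current ammo, and SpawnSnowball rolls it to flag each BP_Projectile as critical.
; Reload refills to max; the spawn-point array built on BeginPlay is unused by firing.
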(event EventBeginPlay
  (bind _asbp_fpscharacter (Utilities|Casting|CastToBP_FPSCharacter (Game|GetPlayerCharacter 0)))
  (Variables|Default|SetFPSPlayerRef _asbp_fpscharacter)
  ;[0.15 0.15 0.15 0.5] CHECK WITH DANNY
  (Variables|Default|SetMultifireSpawnPoints (Utilities|Array|MakeArray (Transformation|GetWorldTransform (Variables|Default|GetSecondaryFire1)) (Transformation|GetWorldTransform (Variables|Default|GetSecondaryFire2)) (Transformation|GetWorldTransform (Variables|Default|GetSecondaryFire3)))))

(event EventReload
  (|CallParentFunction)
  (Variables|Default|SetCurrentAmmo (Variables|Default|GetMaxAmmo)))

(event EventSingleShoot
  (|CallParentFunction)
  (if (Variables|/Game/FPS/Blueprint/Player/BP_FPSCharacter.BP_FPSCharacter_C|GetCrit%20Ability (Variables|Default|GetFPSPlayerRef))
    (Variables|Default|SetCritChance (+ 50 (Variables|Default|GetCurrentAmmo))))
  (if (> (Variables|Default|GetCurrentAmmo) 0)
    (if (Variables|/Game/FPS/Blueprint/Player/BP_FPSCharacter.BP_FPSCharacter_C|GetAmmoAbility (Variables|Default|GetFPSPlayerRef))
      ;[0.15 0.15 0.15 0.5] Ammo Update
      (if (> (Math|Random|RandomInteger 4) 0)
        (Development|PrintString "Ammo Conserved!")
        (else
          (bind _result (Math|Integer|DecrementInt (Variables|Default|GetCurrentAmmo) :!label _label)
            (:%20%20
              _))))
      (else
        (goto _label)))
    (Development|PrintString (Utilities|String|ToString(Integer) _result))
    (CallFunction|SpawnSnowball (Transformation|GetWorldTransform (Variables|Default|GetPrimaryFire)))
    (else
      (Development|PrintString "Out of Ammo"))))

(event EventSpreadShoot
  (|CallParentFunction)
  (if (Variables|/Game/FPS/Blueprint/Player/BP_FPSCharacter.BP_FPSCharacter_C|GetCrit%20Ability (Variables|Default|GetFPSPlayerRef))
    (Variables|Default|SetCritChance (+ 50 (Variables|Default|GetCurrentAmmo))))
  (if (> (Variables|Default|GetCurrentAmmo) 11)
    (if (Variables|/Game/FPS/Blueprint/Player/BP_FPSCharacter.BP_FPSCharacter_C|GetAmmoAbility (Variables|Default|GetFPSPlayerRef))
      ;[0.15 0.15 0.15 0.5] Ammo Update
      (if (> (Math|Random|RandomInteger 4) 0)
        (Development|PrintString "Ammo Conserved!")
        (else
          (bind _output_get (Variables|Default|SetCurrentAmmo (- (Variables|Default|GetCurrentAmmo) 12) :!label _label))))
      (else
        (goto _label)))
    (Development|PrintString (Utilities|String|ToString(Integer) _output_get))
    (CallFunction|SpawnSnowball (Transformation|GetWorldTransform (Variables|Default|GetSecondaryFire1)))
    (CallFunction|SpawnSnowball (Transformation|GetWorldTransform (Variables|Default|GetSecondaryFire2)))
    (CallFunction|SpawnSnowball (Transformation|GetWorldTransform (Variables|Default|GetSecondaryFire3)))
    (CallFunction|SpawnSnowball (Transformation|GetWorldTransform (Variables|Default|GetSecondaryFire4)))
    (CallFunction|SpawnSnowball (Transformation|GetWorldTransform (Variables|Default|GetSecondaryFire5)))
    (CallFunction|SpawnSnowball (Transformation|GetWorldTransform (Variables|Default|GetSecondaryFire6)))
    (else
      (Development|PrintString "Not Enough Ammo"))))

(fn ConstructionScript)

(fn InheritSingleShoot
  (|CallParentFunction))

(fn InheritReload
  (|CallParentFunction))

(fn InheritSpreadShoot
  (|CallParentFunction))

(fn SpawnSnowball
  (params (SpawnPoint :type Transform))
  (bind _crit (CallFunction|CritChanceCheck (Variables|Default|GetCritChance)))
  (bind _returnvalue (Game|SpawnActorfromClass "/Game/FPS/Blueprint/Guns/BP_Projectile.BP_Projectile_C" SpawnPoint "Undefined" "MultiplyWithRoot" 0 0))
  (Variables|/Game/FPS/Blueprint/Guns/BP_Projectile.BP_Projectile_C|SetCriticalHit _returnvalue _crit))