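; BP_Gun is a base gun Blueprint that defines shooting, spread shooting and reload actions for weapons.
; Each action event forwards to an Inherit function, apparently meant for child overrides; both shoot functions are empty and reload only prints a message.
; Helper functions double a given max ammo, roll a percentage crit chance with debug prints, and pass a crit chance value through unchanged.
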(event EventSpreadshoot
  (CallFunction|InheritSpreadShoot))

(event EventSingleShoot
  (CallFunction|InheritSingleShoot))

(event EventReload
  (CallFunction|InheritReload))

(fn ConstructionScript)

(fn InheritSingleShoot)

(fn InheritReload
  (Development|PrintString "Gun Is Reloading..."))

(fn InheritSpreadShoot)

(fn DoubleMaxAmmo
  (params (MaxAmmo :type Integer))
  (bind _output_get (Variables|Default|SetMaxAmmo (* MaxAmmo 2)))
  (return _output_get))

(fn CritChanceCheck
  (params (CritChance :type Integer))
  (if (< (Math|Random|RandomInteger 99) CritChance)
    (Development|PrintString "Crit")
    (return true)
    (else
      (Development|PrintString "No Crit")
      (return false))))

(fn SetCritChance
  (params (Crit%20Chance :type Integer))
  (bind _output_get (Variables|Default|SetCritChance Crit%20Chance))
  (return _output_get))