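; BP_Projectile is a gun projectile for the FPS game that damages what it hits and explodes.
; When its Projectile component activates, it copies ProjectileSpeed into that component's initial and max speed.
; A hit on ProjectileCollision applies ProjectileDamage to the other actor, doubled through DoubleDamage when CriticalHit is set.
; It then spawns an explosion emitter at the impact point and destroys itself.
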(event OnComponentHit(ProjectileCollision)
  (params (HitComponent :type Primitive%20Component%20Object%20Reference) (OtherActor :type Actor%20Object%20Reference) (OtherComp :type Primitive%20Component%20Object%20Reference) (NormalImpulse :type Vector :default "0, 0, 0") (Hit :type Hit%20Result%20Structure%20%28by%20ref%29))
  ;[0.15 0.15 0.15 0.5] Collision
  (if (Variables|Default|GetCriticalHit)
    (bind _doubleprojectiledamage (CallFunction|DoubleDamage))
    (Game|Damage|ApplyDamage OtherActor _doubleprojectiledamage 0 0)
    (else
      (Game|Damage|ApplyDamage OtherActor (Variables|Default|GetProjectileDamage) 0 0)))
  (Effects|SpawnEmitteratLocation "/Game/StarterContent/Particles/P_Explosion.P_Explosion" (.location Hit))
  (Actor|DestroyActor))

(event OnComponentActivated(Projectile)
  (params (Component :type Actor%20Component%20Object%20Reference) (bReset :type Boolean))
  (bind _projectile (Variables|Default|GetProjectile))
  ;[0.15 0.15 0.15 0.5] Projectile Speed
  (Variables|/Script/Engine.ProjectileMovementComponent|SetInitialSpeed _projectile (Variables|Default|GetProjectileSpeed))
  (Variables|/Script/Engine.ProjectileMovementComponent|SetMaxSpeed _projectile (Variables|Default|GetProjectileSpeed)))

(fn ConstructionScript)

(fn DoubleDamage
  (return (* (Variables|Default|GetProjectileDamage) 2.0)))