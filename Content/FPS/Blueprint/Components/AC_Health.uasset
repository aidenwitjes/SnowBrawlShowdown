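; Health component for FPS actors that tracks health within a min and max range and initializes to full on BeginPlay.
; Heal, Damage, HealFull and Kill route through SetHealth, which clamps the value and fires the OnHealthChanged dispatcher.
; Heal and Damage reject non-positive amounts with a printed warning.
; Helpers report death and normalized health, and DoubleMaxHealth doubles a max value and sets health to it.
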(event EventBeginPlay
  (CallFunction|Init (Variables|Default|GetMinHealth) (Variables|Default|GetMaxHealth)))

(fn Heal
  (params (HealAmount :type Float%20%28double-precision%29))
  (if (> HealAmount 0.0)
    (CallFunction|SetHealth (+ (CallFunction|GetHealth) HealAmount))
    (else
      (Development|PrintString "Heal Value Must Be Positive"))))

(fn GetHealth
  (return (Variables|Default|GetHealth)))

(fn SetHealth
  (params (UpdatedHealth :type Float%20%28double-precision%29))
  (bind _output_get (Variables|Default|SetHealth (CallFunction|ClampHealth UpdatedHealth)))
  (Default|CallOnHealthChanged (Variables|Default|GetHealth) (Variables|Default|GetMaxHealth))
  (return _output_get))

(fn GetMaxHealth
  (return (Variables|Default|GetMaxHealth)))

(fn ClampHealth
  (params (Value :type Float%20%28double-precision%29))
  (return (Math|Float|Clamp(Float) Value (Variables|Default|GetMinHealth) (Variables|Default|GetMaxHealth))))

(fn Damage
  (params (Damage%20Amount :type Float%20%28double-precision%29))
  (if (> Damage%20Amount 0.0)
    (CallFunction|SetHealth (- (CallFunction|GetHealth) Damage%20Amount))
    (else
      (Development|PrintString "Damage Value Must Be Positive"))))

(fn IsDead
  (return (<= (CallFunction|GetHealth) (Variables|Default|GetMinHealth))))

(fn GetNormalizedHealth
  (return (Math|Float|Clamp(Float) (/ (CallFunction|GetHealth) (Variables|Default|GetMaxHealth)))))

(fn HealFull
  (CallFunction|Heal (Variables|Default|GetMaxHealth)))

(fn Kill
  (CallFunction|Damage (Variables|Default|GetMaxHealth)))

(fn Init
  (params (New%20Min%20Health :type Float%20%28double-precision%29) (New%20Max%20Health :type Float%20%28double-precision%29))
  (Variables|Default|SetMinHealth New%20Min%20Health)
  (bind _output_get (Variables|Default|SetMaxHealth New%20Max%20Health))
  (CallFunction|SetHealth _output_get))

(fn DoubleMaxHealth
  (params (Max%20Health :type Float%20%28double-precision%29))
  (bind _output_get (Variables|Default|SetMaxHealth (* Max%20Health 2.0)))
  (bind _health (CallFunction|SetHealth _output_get))
  (return _health))