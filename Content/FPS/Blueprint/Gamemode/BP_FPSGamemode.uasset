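; BP_FPSGamemode is the FPS game mode that initializes the player character and owns the HUD, score and wave timer.
; BeginPlay caches and initializes BP_FPSCharacter, then SetupUI creates WBP_GameMenu, sets game-only input and zeroes the score display.
; AddScore updates the score text, while a temporary Tick-plus-Delay counter drives the timer roughly each second, regardless of wave phase.
; Upgrade menu creation is present but never runs.
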(event EventBeginPlay
  ;[0.15 0.15 0.15 0.5] Setting The Gamemode on Play
  (Development|PrintString "Spawning BP_FPSGamemode")
  (bind _asbp_fpscharacter (Utilities|Casting|CastToBP_FPSCharacter (Game|GetPlayerCharacter 0)))
  (Variables|Default|SetFPSPlayerRef _asbp_fpscharacter)
  (Default|Initialize _asbp_fpscharacter)
  (CallFunction|SetupUI))

(event EventTick
  (params (DeltaSeconds :type Float%20%28single-precision%29))
  ;[0.15 0.15 0.15 0.5] Temporary Timer (NEEDS UPDATING TO ONLY COUNT DURING THE WAVE PHASE)
  (CallFunction|SetTimer (stale _result))
  (Utilities|FlowControl|Delay 1.0)
  (bind _result (Math|Integer|IncrementInt (Variables|Default|GetWaveTimer))))

(fn ConstructionScript)

(fn SetTimer
  (params (Timer :type Integer))
  (Rendering|Components|TextRender|SetText (Variables|/Game/FPS/Blueprint/GUI/WBP_GameMenu.WBP_GameMenu_C|GetTextTimer (Variables|Default|GetGameMenuRef)) (Utilities|Text|ToText(String) (Utilities|String|Append "Wave Timer: " (Utilities|String|ToString(Integer) Timer)))))

(fn SetScore
  (params (Score :type Integer))
  (Rendering|Components|TextRender|SetText (Variables|/Game/FPS/Blueprint/GUI/WBP_GameMenu.WBP_GameMenu_C|GetTextScore (Variables|Default|GetGameMenuRef)) (Utilities|Text|ToText(String) (Utilities|String|Append "Score: " (Utilities|String|ToString(Integer) Score)))))

(fn AddScore
  (params (PointsToAdd :type Integer))
  (bind _output_get (Variables|Default|SetScore (+ (Variables|Default|GetScore) PointsToAdd)))
  (CallFunction|SetScore _output_get))

(fn SetupUI
  (bind _returnvalue (Game|GetPlayerController 0))
  (bind _returnvalue_2 (UserInterface|CreateWidget "/Game/FPS/Blueprint/GUI/WBP_GameMenu.WBP_GameMenu_C"))
  (bind _output_get (Variables|Default|SetGameMenuRef _returnvalue_2))
  (UserInterface|Viewport|AddtoViewport _output_get 0)
  (Input|SetInputModeGameOnly _returnvalue false)
  (Variables|/Script/Engine.PlayerController|SetbShowMouseCursor _returnvalue false)
  (CallFunction|SetScore))