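; Snow mound interactable that marks where the FPS character is allowed to reload.
; On BeginPlay it sets the reload prompt text and its interactable system name, then runs the parent interactable logic.
; Overlap begin and end call the parent handlers, then toggle CanReload on the overlapping BP_FPSCharacter, so the flag is on only while in range.
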(event EventBeginPlay
  ;[0.15 0.15 0.15 0.5] Updates Interaction Prompt Text
  (Variables|Default|SetPromptText "Press \"R\" to Reload")
  (Variables|Default|SetInteractableSystemName "SnowMound")
  (|CallParentFunction))

(event Collision|EventActorEndOverlap
  (params (OtherActor :type Actor%20Object%20Reference))
  ;[0.15 0.15 0.15 0.5] SnowMound Out of Range Interaction
  (|CallParentFunction OtherActor)
  (bind _asbp_fpscharacter (Utilities|Casting|CastToBP_FPSCharacter OtherActor))
  (Variables|/Game/FPS/Blueprint/Player/BP_FPSCharacter.BP_FPSCharacter_C|SetCanReload _asbp_fpscharacter false))

(event Collision|EventActorBeginOverlap
  (params (OtherActor :type Actor%20Object%20Reference))
  ;[0.15 0.15 0.15 0.5] SnowMound Overlap Interaction
  (|CallParentFunction OtherActor)
  (bind _asbp_fpscharacter (Utilities|Casting|CastToBP_FPSCharacter OtherActor))
  (Variables|/Game/FPS/Blueprint/Player/BP_FPSCharacter.BP_FPSCharacter_C|SetCanReload _asbp_fpscharacter true))

(fn ConstructionScript
  (|CallParentFunction))